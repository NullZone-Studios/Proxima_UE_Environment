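; BP_Planet is a template actor for a rotating planet with cloud and atmosphere layers.
; The construction script applies configurable materials to the Planet, Clouds and Atmosphere components.
; Each tick, the Planet component rotates locally in yaw by RotationSpeed scaled by delta time for frame-rate-independent spin.
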(event EventBeginPlay)

(event Collision|EventActorBeginOverlap
  (params (OtherActor :type Actor%20Object%20Reference)))

(event EventTick
  (params (DeltaSeconds :type Float%20%28single-precision%29))
  (Transformation|AddLocalRotation (Variables|Default|GetPlanet) (Math|Rotator|MakeRotator 0.0 0.0 (* DeltaSeconds (Variables|Default|GetRotation%20Speed))) false false))

(fn ConstructionScript
  (Rendering|Material|SetMaterial (Variables|Default|GetPlanet) 0 (Variables|Default|GetPlanet%20Material))
  (Rendering|Material|SetMaterial (Variables|Default|GetClouds) 0 (Variables|Default|GetCloud%20Material))
  (Rendering|Material|SetMaterial (Variables|Default|GetAtmosphere) 0 (Variables|Default|GetAtmosphere%20Material)))