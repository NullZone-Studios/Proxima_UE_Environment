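; Player movement component that handles walking, sprinting and camera zoom for the owning PlayerCharacter through Enhanced Input.
; InitializeInput caches the character, spring arm and controller, then adds the default mapping context.
; Move input is applied along world X/Y axes, normalized and independent of camera rotation.
; Sprint and zoom inputs set targets, with zoom clamped, and Tick smoothly interpolates walk speed and arm length toward them.
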(event Custom|InitializeInput
  (bind _returnvalue (Components|GetOwner))
  ;[1 1 1] Input Mapping & References Setup
  (Utilities|FlowControl|Sequence
    (:then_0
      (bind _asplayer_character (Utilities|Casting|CastToPlayerCharacter _returnvalue))
      (Variables|Default|SetParent _asplayer_character)
      (Variables|Default|SetParentSpringArm (Actor|GetComponentbyClass _returnvalue "/Script/Engine.SpringArmComponent")))
    (:then_1
      (bind _asplayer_controller (Utilities|Casting|CastToPlayerController (Pawn|GetController (Variables|Default|GetParent))))
      (Input|AddMappingContext (PlayerController|LocalPlayerSubsystems|GetEnhancedInputLocalPlayerSubsystem _asplayer_controller) "/Game/Blueprints/Input/IMC_Default.IMC_Default" 0 "(bIgnoreAllPressedKeysUntilRelease=True,bForceImmediately=False,bNotifyUserSettings=False)"))))

(event Input|EnhancedActionEvents|EnhancedInputActionIA_Move
  (params (ActionValue :type Vector%202D%20Structure) (ElapsedSeconds :type Float%20%28double-precision%29) (TriggeredSeconds :type Float%20%28double-precision%29) (InputAction :type Input%20Action%20Object%20Reference :default "/Game/Blueprints/Input/IA_Move.IA_Move"))
  ;[1 0.9047 0.2582] Movement
  (Pawn|Input|AddMovementInput (Variables|Default|GetParent) (Math|Vector|Normalize (Math|Vector|MakeVector (.x ActionValue) (.y ActionValue) 0.0)) 1.0 false))

(event Input|EnhancedActionEvents|EnhancedInputActionIA_Sprint
  (params (ActionValue :type Boolean) (ElapsedSeconds :type Float%20%28double-precision%29) (TriggeredSeconds :type Float%20%28double-precision%29) (InputAction :type Input%20Action%20Object%20Reference :default "/Game/Blueprints/Input/IA_Sprint.IA_Sprint"))
  ;[1 0.9047 0.2582] Movement
  (:Triggered
    (Variables|Default|SetTargetSpeed (Variables|Default|GetBaseRunningSpeed)))
  (:Completed
    (Variables|Default|SetTargetSpeed (Variables|Default|GetBaseWalkingSpeed))))

(event Input|EnhancedActionEvents|EnhancedInputActionIA_Zoom
  (params (ActionValue :type Float%20%28double-precision%29) (ElapsedSeconds :type Float%20%28double-precision%29) (TriggeredSeconds :type Float%20%28double-precision%29) (InputAction :type Input%20Action%20Object%20Reference :default "/Game/Blueprints/Input/IA_Zoom.IA_Zoom"))
  ;[1 0.9047 0.2582] Zoom
  (bind _output_get (Variables|Default|SetTargetZoomLength (Math|Float|Clamp(Float) (+ ActionValue (Variables|Default|GetTargetZoomLength)) 5e+02 1.5e+03))))

(event EventTick
  (params (DeltaSeconds :type Float%20%28single-precision%29))
  (bind _parent (Variables|Default|GetParent))
  (bind _targetspeed (Variables|Default|GetTargetSpeed))
  (bind _parentspringarm (Variables|Default|GetParentSpringArm))
  (bind _charactermovement (Variables|/Script/Engine.Character|GetCharacterMovement _parent))
  ;[1 0.9047 0.2582] Zoom
  (if (!= (Variables|Default|GetTargetZoomLength) (Variables|/Script/Engine.SpringArmComponent|GetTargetArmLength _parentspringarm))
    (Variables|/Script/Engine.SpringArmComponent|SetTargetArmLength _parentspringarm (Math|Interpolation|FInterpTo (Variables|/Script/Engine.SpringArmComponent|GetTargetArmLength _parentspringarm) (stale Input|EnhancedActionEvents|EnhancedInputActionIA_Zoom _output_get) (Utilities|Time|GetWorldDeltaSeconds) (Variables|Default|GetZoomSpeed))))
  ;[0.5677 0.5677 0.5677] Interpolation between walking and running
  (if (!= (Variables|/Script/Engine.CharacterMovementComponent|GetMaxWalkSpeed _charactermovement) _targetspeed)
    (Variables|/Script/Engine.CharacterMovementComponent|SetMaxWalkSpeed _charactermovement (Math|Interpolation|FInterpTo (Variables|/Script/Engine.CharacterMovementComponent|GetMaxWalkSpeed _charactermovement) _targetspeed DeltaSeconds 3.0))))