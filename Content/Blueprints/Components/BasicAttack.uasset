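; BasicAttack is a component that gives the player character a basic attack by spawning an ability actor.
; Setup caches the owning BP_NewPlayer and adds the IMC_Default Enhanced Input mapping context to its player controller.
; BasicAttack_Event spawns the Ability class at the player's transform, passing the player reference to the spawned actor.
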(event Custom|Setup
  ;[0.15 0.15 0.15 0.5] Setup
  (Utilities|FlowControl|Sequence
    (:then_0
      (bind _asbp_new_player (Utilities|Casting|CastToBP_NewPlayer (Components|GetOwner)))
      (Variables|Default|SetPlayerRef _asbp_new_player))
    (:then_1
      (bind _asplayer_controller (Utilities|Casting|CastToPlayerController (Pawn|GetController (Variables|Default|GetPlayerRef))))
      (Input|AddMappingContext (PlayerController|LocalPlayerSubsystems|GetEnhancedInputLocalPlayerSubsystem _asplayer_controller) "/Game/Blueprints/Input/IMC_Default.IMC_Default" 0 "(bIgnoreAllPressedKeysUntilRelease=True,bForceImmediately=False,bNotifyUserSettings=False)"))))

(event Custom|BasicAttack_Event
  (bind _playerref (Variables|Default|GetPlayerRef))
  (Game|SpawnActorfromClass (Variables|Default|GetAbility) (Transformation|GetActorTransform _playerref) "Undefined" "MultiplyWithRoot" 0 _playerref 0))