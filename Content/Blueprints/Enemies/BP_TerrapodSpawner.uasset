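; Enemy spawner that periodically spawns BP_Terrapod near itself while the BaseEnemy count is at or below MaxSpawns.
; BeginPlay randomizes the spawn delay once when the range is valid, and Tick counts it down.
; RandomLocation capsule-traces vertically around random reachable navmesh points, then projects the hit back onto navigation.
; Failures retry recursively while CurrentAttempt is below SpawnAttempts, but the counter is never incremented here.
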(event EventBeginPlay
  (bind _spawn_delay_min (Variables|Default|GetSpawn%20Delay%20Min))
  (bind _spawn_delay_max (Variables|Default|GetSpawn%20Delay%20Max))
  ;[0.15 0.15 0.15 0.5] Setup Spawn delay
  (if (< _spawn_delay_min _spawn_delay_max)
    (Variables|Default|SetSpawn%20Delay (Math|Random|RandomFloatinRange _spawn_delay_min _spawn_delay_max))))

(event EventTick
  (params (DeltaSeconds :type Float%20%28single-precision%29))
  ;[0.15 0.15 0.15 0.5] Spawn Logic
  (if (< (Variables|Default|GetSpawn%20Timer) 0.0)
    (bind _outactors (Actor|GetAllActorsOfClass "/Script/UE_Environment.BaseEnemy"))
    (if (<= (Utilities|Array|Length _outactors) (Variables|Default|GetMax%20Spawns))
      (Variables|Default|SetCurrent%20Attempt 0)
      (bind (_spawnlocation _success) (CallFunction|RandomLocation))
      (if _success
        (Game|SpawnActorfromClass "/Game/Blueprints/Enemies/BP_Terrapod.BP_Terrapod_C" (Math|Conversions|ToTransform(Vector) _spawnlocation) "Undefined" "MultiplyWithRoot" 0 0)))
    (Variables|Default|SetSpawn%20Timer (Variables|Default|GetSpawn%20Delay))
    (else
      (Variables|Default|SetSpawn%20Timer (- (Variables|Default|GetSpawn%20Timer) DeltaSeconds)))))

(fn ConstructionScript)

(fn RandomLocation
  (bind _returnvalue (Transformation|GetActorLocation))
  (bind _randomlocation (AI|Navigation|GetRandomReachablePointinRadius _returnvalue 1e+03 0 0))
  (bind (_outhit _returnvalue_2) (Collision|CapsuleTraceByChannel (+ _randomlocation "0.000000,0.000000,3000.000000") (- _randomlocation "0.000000,0.000000,5000.000000") 4e+01 9e+01 "TraceTypeQuery1" false 0 "None"))
  (if _returnvalue_2
    (if (.ReturnValue (AI|Navigation|ProjectPointtoNavigation (+ (.location _outhit) "0.000000,0.000000,30.000000") 0 0 "0, 0, 0"))
      (return (.ProjectedLocation (AI|Navigation|ProjectPointtoNavigation (+ (.location _outhit) "0.000000,0.000000,30.000000") 0 0 "0, 0, 0")) true)
      (else
        _)))
  (if (< (Variables|Default|GetCurrent%20Attempt) (Variables|Default|GetSpawn%20Attempts))
    (bind (_spawnlocation _success) (CallFunction|RandomLocation))
    (return _spawnlocation _success)
    (else
      (return "0, 0, 0" false))))