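; BP_Terrapod is an enemy that chases the player once it sees a pawn.
; PawnSensing sets IsSeeinPlayer on any seen pawn, without a player check or reset here, then FollowPlayer issues AI MoveTo toward player 0.
; Tick sets IsMoving from last update velocity, inverted relative to its name: true at zero velocity.
; An unconnected GainXP call on the player character never runs.
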(event OnSeePawn(PawnSensing)
  (params (Pawn :type Pawn%20Object%20Reference))
  (Variables|Default|SetIsSeeinPlayer? true)
  (CallFunction|FollowPlayer))

(event Custom|FollowPlayer
  (if (Variables|Default|GetIsSeeinPlayer?)
    (AI|AIMoveTo self "0, 0, 0" (Game|GetPlayerCharacter 0) 5.0 false)))

(event EventBeginPlay)

(event Collision|EventActorBeginOverlap
  (params (OtherActor :type Actor%20Object%20Reference)))

(event EventTick
  (params (DeltaSeconds :type Float%20%28single-precision%29))
  (if (Utilities|Operators|EqualEqual :A (Pawn|Components|CharacterMovement|GetLastUpdateVelocity (Variables|Character|GetCharacterMovement)))
    (Variables|Default|SetIsMoving true)
    (else
      (Variables|Default|SetIsMoving false))))

(fn ConstructionScript)