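; Player hero Blueprint that handles health, abilities and XP leveling, and creates its HUD on BeginPlay.
; Enhanced Input actions trigger basic attack, two abilities and ultimate on separate hero components, gated by cooldowns updated on Tick.
; Damage passes through an invulnerability check that also updates on Tick, while Death is an empty stub.
; XP gain applies a bonus, scales the next-level threshold on level-up and activates an emitter.
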(event Custom|TakingDamage_Event
  (params (Damage :type Float%20%28double-precision%29) (Circumvent%20Invulnerability :type Boolean))
  (bind _returnvalue (Class|PlayerCharacter|TakeDamage Damage (Class|PlayerCharacter|IsInvulnerable) Circumvent%20Invulnerability))
  (if _returnvalue
    (Class|PlayerCharacter|ResetInvulnerability))
  (if (Class|PlayerCharacter|IsAlive)
    (CallFunction|Death)))

(event Input|EnhancedActionEvents|EnhancedInputActionIA_Attack
  (params (ActionValue :type Boolean) (ElapsedSeconds :type Float%20%28double-precision%29) (TriggeredSeconds :type Float%20%28double-precision%29) (InputAction :type Input%20Action%20Object%20Reference :default "/Game/Blueprints/Input/IA_Attack.IA_Attack"))
  ;[0.15 0.15 0.15 0.5] Basic Attack
  (if (Class|PlayerCharacter|IsAttackOffCooldown)
    (Default|BasicAttackEvent (Variables|Default|GetHero%20Basic%20Attack))
    (Class|PlayerCharacter|ResetAttackCooldown)))

(event Input|EnhancedActionEvents|EnhancedInputActionIA_Ability1
  (params (ActionValue :type Boolean) (ElapsedSeconds :type Float%20%28double-precision%29) (TriggeredSeconds :type Float%20%28double-precision%29) (InputAction :type Input%20Action%20Object%20Reference :default "/Game/Blueprints/Input/IA_Ability1.IA_Ability1"))
  ;[0.15 0.15 0.15 0.5] Ability 1
  (if (Class|PlayerCharacter|IsAbility1OffCooldown)
    (Default|AbilityEvent (Variables|Default|GetHero%20Ability%201))))

(event Input|EnhancedActionEvents|EnhancedInputActionIA_Ability2
  (params (ActionValue :type Boolean) (ElapsedSeconds :type Float%20%28double-precision%29) (TriggeredSeconds :type Float%20%28double-precision%29) (InputAction :type Input%20Action%20Object%20Reference :default "/Game/Blueprints/Input/IA_Ability2.IA_Ability2"))
  ;[0.15 0.15 0.15 0.5] Ability 2
  (if (Class|PlayerCharacter|IsAbility2OffCooldown)
    (Default|AbilityEvent (Variables|Default|GetHero%20Ability%202))))

(event Input|EnhancedActionEvents|EnhancedInputActionIA_Ultimate
  (params (ActionValue :type Boolean) (ElapsedSeconds :type Float%20%28double-precision%29) (TriggeredSeconds :type Float%20%28double-precision%29) (InputAction :type Input%20Action%20Object%20Reference :default "/Game/Blueprints/Input/IA_Ultimate.IA_Ultimate"))
  ;[0.15 0.15 0.15 0.5] Ultimate
  (if (Class|PlayerCharacter|IsAbility3OffCooldown)
    (Default|AbilityEvent (Variables|Default|GetHero%20Ultimate))))

(event EventBeginPlay
  (Utilities|IsValid (Variables|Default|GetHUD_Player)
    (:Is%20Valid
      _)
    (:Is%20Not%20Valid
      (bind _returnvalue (UserInterface|CreateWidget "/Game/UI/HUD_Player.HUD_Player_C"))
      (UserInterface|Viewport|AddtoViewport _returnvalue 0)
      (bind _output_get (Variables|Default|SetHUD_Player _returnvalue))
      (Utilities|IsValid (Variables|/Game/UI/HUD_Player.HUD_Player_C|GetCharacterReference _output_get)
        (:Is%20Valid
          _)
        (:Is%20Not%20Valid
          (Variables|/Game/UI/HUD_Player.HUD_Player_C|SetCharacterReference _output_get self)))))
  (Variables|/Game/UI/HUD_Player.HUD_Player_C|SetDisplayedHealth _output_get (Variables|Default|GetMaxHealth))
  (Default|InitializeInput (Variables|Components|GetPlayerMovement))
  (Variables|/Game/UI/HUD_Player.HUD_Player_C|SetDisplayedXP _output_get (Variables|Default|GetXP))
  (Class|PlayerCharacter|UpdateCooldownStats)
  (Variables|Default|SetHealth (Variables|Default|GetMaxHealth))
  (CallFunction|AwakeAbilities))

(event Collision|EventActorBeginOverlap
  (params (OtherActor :type Actor%20Object%20Reference)))

(event EventTick
  (params (DeltaSeconds :type Float%20%28single-precision%29))
  (Class|PlayerCharacter|UpdateCooldowns DeltaSeconds)
  (Class|PlayerCharacter|UpdateInvulnerability DeltaSeconds))

(fn ConstructionScript)

(fn LevelUpCheck
  (if (>= (Variables|Default|GetXP) (Variables|Default|GetNextLevelXP))
    (Variables|Default|SetXP (- (Variables|Default|GetXP) (Variables|Default|GetNextLevelXP)))
    (Variables|Default|SetNextLevelXP (* (Variables|Default|GetNextLevelXP) (Variables|Default|GetLevelUpMultiplier)))
    (Math|Integer|IncrementInt (Variables|Default|GetLevel)
      (:%20%20
        (return true)))
    (else
      (return false))))

(fn XPGain
  (params (XP :type Float%20%28double-precision%29))
  (Variables|Default|SetXP (+ (* XP (Variables|Default|GetXP_Gain)) (Variables|Default|GetXP)))
  (bind _issuccesfull (CallFunction|LevelUpCheck))
  (if _issuccesfull
    (Components|Activation|Activate (Variables|Default|GetLevelUpEmitter) _issuccesfull)))

(fn Death)

(fn AwakeAbilities
  (Default|Setup (Variables|Default|GetHero%20Basic%20Attack))
  (Default|Setup (Variables|Default|GetHero%20Ability%201))
  (Default|Setup (Variables|Default|GetHero%20Ability%202))
  (Default|Setup (Variables|Default|GetHero%20Ultimate)))